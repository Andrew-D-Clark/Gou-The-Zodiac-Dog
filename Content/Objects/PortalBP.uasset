(event OnComponentBeginOverlap(Cube)
  (params (OverlappedComponent :type Primitive%20Component%20Object%20Reference) (OtherActor :type Actor%20Object%20Reference) (OtherComp :type Primitive%20Component%20Object%20Reference) (OtherBodyIndex :type Integer) (bFromSweep :type Boolean) (SweepResult :type Hit%20Result%20Structure%20%28by%20ref%29))
  (if (Variables|Default|GetIsPortalActive?)
    (bind _asgou_zodiac_dog_character (Utilities|Casting|CastToGouZodiacDogCharacter (stale OnComponentEndOverlap(Cube) OtherActor)))
    (Game|OpenLevel(byName) "ThankYou_Screen")
    (UserInterface|CreateWidget "/Game/UMG_Assets/ThankYou/ThankYou_Widget.ThankYou_Widget_C" (Game|GetPlayerController 0))))

(event OnComponentEndOverlap(Cube)
  (params (OverlappedComponent :type Primitive%20Component%20Object%20Reference) (OtherActor :type Actor%20Object%20Reference) (OtherComp :type Primitive%20Component%20Object%20Reference) (OtherBodyIndex :type Integer))
  (if (Variables|Default|GetIsPortalActive?)
    (bind _asgou_zodiac_dog_character (Utilities|Casting|CastToGouZodiacDogCharacter OtherActor))
    (Game|OpenLevel(byName) "ThankYou_Screen")
    (UserInterface|CreateWidget "/Game/UMG_Assets/ThankYou/ThankYou_Widget.ThankYou_Widget_C" (Game|GetPlayerController 0))))

(event EventBeginPlay)

(event Collision|EventActorBeginOverlap
  (params (OtherActor :type Actor%20Object%20Reference)))

(event EventTick
  (params (DeltaSeconds :type Float%20%28single-precision%29))
  (Utilities|FlowControl|Delay 1.0)
  (if (Variables|Default|GetIsPortalActive?)
    (Rendering|SetVisibility (Variables|Default|GetCube) true false)))

(fn ConstructionScript)