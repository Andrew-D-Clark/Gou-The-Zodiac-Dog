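; Treasure chest that swings its lid open when the GouZodiacDogCharacter enters its trigger and hands out a rabbit medallion.
; The LidOpening timeline drives the lid's roll, and a DoOnce on its update waits briefly, then plays a bell, spawns an effect and spawns the medallion at SpawnLocation.
; An E-key FlipFlop toggles the lid, but the EnableInput call is unwired and leaving the trigger disables input.
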(event OnComponentBeginOverlap(TB_TreasureChest)
  (params (OverlappedComponent :type Primitive%20Component%20Object%20Reference) (OtherActor :type Actor%20Object%20Reference) (OtherComp :type Primitive%20Component%20Object%20Reference) (OtherBodyIndex :type Integer) (bFromSweep :type Boolean) (SweepResult :type Hit%20Result%20Structure%20%28by%20ref%29))
  (Utilities|Casting|CastToGouZodiacDogCharacter OtherActor)
  (bind _lid_float (Timeline|LidOpening Play)
    (:Update
      (Transformation|SetRelativeRotation (Variables|Default|Gettreasurecovertop) (Math|Rotator|MakeRotator _lid_float 0.0 0.0) false false)
      (Utilities|FlowControl|DoOnce false
        (:Completed
          (Utilities|FlowControl|Delay 1.0)
          (Audio|PlaySound2D "/Game/Sounds/Bell__wav_Cue.Bell__wav_Cue")
          (Effects|SpawnEmitteratLocation "/Game/ZodiacAbilities/fx_transform.fx_transform" (Transformation|GetWorldLocation (Variables|Default|GetSpawnLocation)))
          (Game|SpawnActorfromClass "/Game/UMG_Assets/Rabbit_MedallionBP.Rabbit_MedallionBP_C" (Transformation|GetWorldTransform (Variables|Default|GetSpawnLocation)) "Undefined" 0 0))))))

(event OnComponentEndOverlap(TB_TreasureChest)
  (params (OverlappedComponent :type Primitive%20Component%20Object%20Reference) (OtherActor :type Actor%20Object%20Reference) (OtherComp :type Primitive%20Component%20Object%20Reference) (OtherBodyIndex :type Integer))
  (Input|DisableInput (Game|GetPlayerController 0)))

(event Collision|EventActorBeginOverlap
  (params (OtherActor :type Actor%20Object%20Reference)))

(event EventTick
  (params (DeltaSeconds :type Float%20%28single-precision%29)))

(event Input|KeyboardEvents|E
  (params (Key :type Key%20Structure))
  (:Pressed
    (Utilities|FlowControl|FlipFlop
      (:A
        (bind _lid_float (Timeline|LidOpening Play)
          (:Update
            (Transformation|SetRelativeRotation (Variables|Default|Gettreasurecovertop) (Math|Rotator|MakeRotator _lid_float 0.0 0.0) false false)
            (Utilities|FlowControl|DoOnce false
              (:Completed
                (Utilities|FlowControl|Delay 1.0)
                (Audio|PlaySound2D "/Game/Sounds/Bell__wav_Cue.Bell__wav_Cue")
                (Effects|SpawnEmitteratLocation "/Game/ZodiacAbilities/fx_transform.fx_transform" (Transformation|GetWorldLocation (Variables|Default|GetSpawnLocation)))
                (Game|SpawnActorfromClass "/Game/UMG_Assets/Rabbit_MedallionBP.Rabbit_MedallionBP_C" (Transformation|GetWorldTransform (Variables|Default|GetSpawnLocation)) "Undefined" 0 0))))))
      (:B
        (Timeline|LidOpening Reverse)))))

(fn ConstructionScript)