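; JadeOrbBP is a health pickup that GouZodiacDogCharacter collects by overlapping it.
; Only when the character's CurrentHealth is below the hardcoded cap does the orb destroy itself and play a 2D health sound.
; It increments the character's JadeOrbCount, and a count of one adds a health point and resets the counter, so one orb heals when starting from zero.
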(event EventBeginPlay)

(event Collision|EventActorBeginOverlap
  (params (OtherActor :type Actor%20Object%20Reference))
  (bind _asgou_zodiac_dog_character (Utilities|Casting|CastToGouZodiacDogCharacter OtherActor))
  (if (< (Variables|/Game/CharacterBPS/ThirdPersonBP/Blueprints/GouZodiacDogCharacter.GouZodiacDogCharacter_C|GetCurrentHealth _asgou_zodiac_dog_character) 3.0)
    (Actor|DestroyActor)
    (Audio|PlaySound2D "/Game/Sounds/health_01_Cue.health_01_Cue")
    (Variables|/Game/CharacterBPS/ThirdPersonBP/Blueprints/GouZodiacDogCharacter.GouZodiacDogCharacter_C|SetJadeOrbCount _asgou_zodiac_dog_character (+ (Variables|/Game/CharacterBPS/ThirdPersonBP/Blueprints/GouZodiacDogCharacter.GouZodiacDogCharacter_C|GetJadeOrbCount _asgou_zodiac_dog_character) 1))
    (if (== (Variables|/Game/CharacterBPS/ThirdPersonBP/Blueprints/GouZodiacDogCharacter.GouZodiacDogCharacter_C|GetJadeOrbCount _asgou_zodiac_dog_character) 1)
      (if (< (Variables|/Game/CharacterBPS/ThirdPersonBP/Blueprints/GouZodiacDogCharacter.GouZodiacDogCharacter_C|GetCurrentHealth _asgou_zodiac_dog_character) 3.0)
        (Variables|/Game/CharacterBPS/ThirdPersonBP/Blueprints/GouZodiacDogCharacter.GouZodiacDogCharacter_C|SetCurrentHealth _asgou_zodiac_dog_character (+ (Variables|/Game/CharacterBPS/ThirdPersonBP/Blueprints/GouZodiacDogCharacter.GouZodiacDogCharacter_C|GetCurrentHealth _asgou_zodiac_dog_character) 1.0)))
      (Variables|/Game/CharacterBPS/ThirdPersonBP/Blueprints/GouZodiacDogCharacter.GouZodiacDogCharacter_C|SetJadeOrbCount _asgou_zodiac_dog_character 0))))

(event EventTick
  (params (DeltaSeconds :type Float%20%28single-precision%29)))

(fn ConstructionScript)