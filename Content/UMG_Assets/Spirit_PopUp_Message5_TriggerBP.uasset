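; Trigger actor that completes the flower delivery to a spirit when the Gou Zodiac dog character overlaps it while holding a flower.
; It sets the character's objective and spirit text option, then adds the Spirit_PopUp_Typewriter widget to the viewport.
; It then clears the flower and curse flags, spawns a Tiger medallion above itself and destroys itself, making it a one-shot trigger.
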(event EventBeginPlay)

(event Collision|EventActorBeginOverlap
  (params (OtherActor :type Actor%20Object%20Reference))
  (bind _asgou_zodiac_dog_character (Utilities|Casting|CastToGouZodiacDogCharacter OtherActor))
  (if (Variables|/Game/CharacterBPS/ThirdPersonBP/Blueprints/GouZodiacDogCharacter.GouZodiacDogCharacter_C|GetHasFlower? _asgou_zodiac_dog_character)
    (Variables|/Game/CharacterBPS/ThirdPersonBP/Blueprints/GouZodiacDogCharacter.GouZodiacDogCharacter_C|SetCurrentObjective _asgou_zodiac_dog_character 4)
    (Variables|/Game/CharacterBPS/ThirdPersonBP/Blueprints/GouZodiacDogCharacter.GouZodiacDogCharacter_C|SetSpiritTextOption _asgou_zodiac_dog_character 1)
    (bind _returnvalue (UserInterface|CreateWidget "/Game/UMG_Assets/Spirit_PopUp_Typewriter.Spirit_PopUp_Typewriter_C"))
    (UserInterface|Viewport|AddtoViewport _returnvalue 0)
    (if (Variables|/Game/CharacterBPS/ThirdPersonBP/Blueprints/GouZodiacDogCharacter.GouZodiacDogCharacter_C|GetHasFlower? _asgou_zodiac_dog_character)
      (Variables|/Game/CharacterBPS/ThirdPersonBP/Blueprints/GouZodiacDogCharacter.GouZodiacDogCharacter_C|SetHasFlower? _asgou_zodiac_dog_character false)
      (Variables|/Game/CharacterBPS/ThirdPersonBP/Blueprints/GouZodiacDogCharacter.GouZodiacDogCharacter_C|SetIsCursed? _asgou_zodiac_dog_character false)
      (Game|SpawnActorfromClass "/Game/UMG_Assets/Tiger_MedallionBP.Tiger_MedallionBP_C" (Math|Conversions|ToTransform(Vector) (Math|Transform|TransformLocation (Math|Conversions|ToTransform(Vector) (Transformation|GetActorLocation)) "0, 0,100.000000")) "Undefined" 0 0)
      (Actor|DestroyActor)
      (Variables|/Game/CharacterBPS/ThirdPersonBP/Blueprints/GouZodiacDogCharacter.GouZodiacDogCharacter_C|SetHasFlower? _asgou_zodiac_dog_character false)
      (Development|PrintString "Flower Set Off"))))

(event EventTick
  (params (DeltaSeconds :type Float%20%28single-precision%29)))

(fn ConstructionScript)