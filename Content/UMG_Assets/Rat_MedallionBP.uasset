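; Rat medallion pickup actor that unlocks Rat selection for the player's GouZodiacDogCharacter.
; On overlap with that character, it sets CanSelectRat, destroys itself, then creates and shows the PickedUp_Rat and Tutorial_Basics widgets.
; Tick spins the medallion mesh around yaw at a steady, frame-rate-independent speed.
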(event EventBeginPlay)

(event Collision|EventActorBeginOverlap
  (params (OtherActor :type Actor%20Object%20Reference))
  (bind _asgou_zodiac_dog_character (Utilities|Casting|CastToGouZodiacDogCharacter OtherActor))
  (Variables|/Game/CharacterBPS/ThirdPersonBP/Blueprints/GouZodiacDogCharacter.GouZodiacDogCharacter_C|SetCanSelectRat? _asgou_zodiac_dog_character true)
  (Actor|DestroyActor)
  (bind _returnvalue (UserInterface|CreateWidget "/Game/UMG_Assets/PickedUp_RatBP.PickedUp_RatBP_C"))
  (bind _returnvalue_2 (UserInterface|CreateWidget "/Game/UMG_Assets/Tutorial/Tutorial_Basics_Widget.Tutorial_Basics_Widget_C"))
  (UserInterface|Viewport|AddtoViewport _returnvalue 0))

(event EventTick
  (params (DeltaSeconds :type Float%20%28single-precision%29))
  (Transformation|AddRelativeRotation (Variables|Default|GetRatMedallion) (Math|Rotator|MakeRotator 0.0 0.0 (* DeltaSeconds 1.8e+02)) false false))

(fn ConstructionScript)