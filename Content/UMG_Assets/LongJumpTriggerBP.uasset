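; Trigger actor that shows the long jump hint and updates the objective when the dog player character reaches it.
; On overlap with a GouZodiacDogCharacter, it adds a new LongJumpHintBP widget to the viewport and sets CurrentObjective to 1.
; Pause, self-destroy, hint removal and timed Jade Emperor text nodes are disconnected, so each overlap adds another widget.
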(event EventBeginPlay)

(event Collision|EventActorBeginOverlap
  (params (OtherActor :type Actor%20Object%20Reference))
  (bind _asgou_zodiac_dog_character (Utilities|Casting|CastToGouZodiacDogCharacter OtherActor))
  (bind _returnvalue (UserInterface|CreateWidget "/Game/UMG_Assets/LongJumpHintBP.LongJumpHintBP_C" (Game|GetPlayerController 0)))
  (UserInterface|Viewport|AddtoViewport _returnvalue 0)
  (Variables|/Game/CharacterBPS/ThirdPersonBP/Blueprints/GouZodiacDogCharacter.GouZodiacDogCharacter_C|SetCurrentObjective _asgou_zodiac_dog_character 1))

(event EventTick
  (params (DeltaSeconds :type Float%20%28single-precision%29)))

(fn ConstructionScript)