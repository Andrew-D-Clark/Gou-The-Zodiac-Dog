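; Spirit_PopUpTriggerBP is a one-shot trigger actor that shows a spirit pop-up and curses the player's zodiac dog character if it lacks the flower.
; On overlap by a GouZodiacDogCharacter without HasFlower, it adds the Spirit_PopUp_Typewriter widget to the viewport, sets IsCursed, updates CurrentObjective and destroys itself.
; Disconnected leftover nodes for delayed Spirit and Jade Emperor text switching never run.
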(event EventBeginPlay)

(event Collision|EventActorBeginOverlap
  (params (OtherActor :type Actor%20Object%20Reference))
  (bind _asgou_zodiac_dog_character (Utilities|Casting|CastToGouZodiacDogCharacter OtherActor))
  (if (not (Variables|/Game/CharacterBPS/ThirdPersonBP/Blueprints/GouZodiacDogCharacter.GouZodiacDogCharacter_C|GetHasFlower? _asgou_zodiac_dog_character))
    (bind _returnvalue (UserInterface|CreateWidget "/Game/UMG_Assets/Spirit_PopUp_Typewriter.Spirit_PopUp_Typewriter_C"))
    (UserInterface|Viewport|AddtoViewport _returnvalue 0)
    (Variables|/Game/CharacterBPS/ThirdPersonBP/Blueprints/GouZodiacDogCharacter.GouZodiacDogCharacter_C|SetIsCursed? _asgou_zodiac_dog_character true)
    (Actor|DestroyActor)
    (Variables|/Game/CharacterBPS/ThirdPersonBP/Blueprints/GouZodiacDogCharacter.GouZodiacDogCharacter_C|SetCurrentObjective _asgou_zodiac_dog_character 8)))

(event EventTick
  (params (DeltaSeconds :type Float%20%28single-precision%29)))

(fn ConstructionScript)