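; Breakable bamboo Blueprint that fractures its Destructible component when a tiger claw actor overlaps it.
; On overlap with tiger_claw_bp, it applies damage at the component's location with an impulse along the player character's forward vector, then enables physics simulation.
; A hit-based radius damage path is left unconnected and never runs.
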(event EventBeginPlay)

(event EventTick
  (params (DeltaSeconds :type Float%20%28single-precision%29)))

(event Collision|EventHit
  (params (MyComp :type Primitive%20Component%20Object%20Reference) (Other :type Actor%20Object%20Reference) (OtherComp :type Primitive%20Component%20Object%20Reference) (bSelfMoved :type Boolean) (HitLocation :type Vector :default "0, 0, 0") (HitNormal :type Vector :default "0, 0, 0") (NormalImpulse :type Vector :default "0, 0, 0") (Hit :type Hit%20Result%20Structure%20%28by%20ref%29)))

(event Collision|EventActorBeginOverlap
  (params (OtherActor :type Actor%20Object%20Reference))
  (bind _destructible (Variables|Default|GetDestructible))
  (bind _astiger_claw_bp (Utilities|Casting|CastTotiger_claw_bp OtherActor))
  (Class|DestructibleComponent|ApplyDamage _destructible 1.0 (Transformation|GetWorldLocation _destructible) (Transformation|GetActorForwardVector (Game|GetPlayerCharacter 0)) 1.0)
  (Physics|SetSimulatePhysics _destructible true))

(fn ConstructionScript)